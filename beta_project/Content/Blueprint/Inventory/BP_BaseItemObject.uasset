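; BP_BaseItemObject is the base inventory item object that exposes an item's size, icon and class to other code.
; GetItemDimention returns the item's Dimension, and GetItemClass returns the class stored for the item.
; GetItemIcon switches between the normal and rotated icon based on the IsRotate flag, so rotated items get their own art.
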(fn `GetItemClass`
  (returns (ItemClass :type "/Game/Blueprint/Inventory/BP_BaseInventoryItem Class Reference"))
  (return (`self.ItemClass`)))

(fn `GetItemDimention`
  (returns (Dimension :type "IntPoint Structure"))
  (return (`self.Dimension`)))

(fn `GetItemIcon`
  (returns (Icon :type "Texture2D Object Reference"))
  (return (select `bool` (`self.IsRotate`) :`false` (`self.Icon`) :`true` (`self.Icon_Rotate`))))
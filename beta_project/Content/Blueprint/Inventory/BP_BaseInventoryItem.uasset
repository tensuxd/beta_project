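; Base world actor for an inventory item that is picked up through an Interact event.
; On BeginPlay it builds a default BP_BaseItemObject if none is valid, storing grid dimensions, placeholder icons and its own class.
; Interact passes that item object to the given inventory component's TryAddItem, prints the result, and on success calls ServerDestroyItem to destroy the actor.
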(event `self.ReceiveBeginPlay`
  (if (not (`KismetSystemLibrary.IsValid` (`self.ItemObject`)))
    (bind _itemobject (`self.Get Default Item Object`))
    (set `self.ItemObject` _itemobject)))

(event `/Game/Blueprint/Inventory/BPI_Interact.Interact`
  (params (InventoryComponent :type "/Game/Blueprint/Inventory/AC_Inventory Object Reference"))
  (bind _added (`/Game/Blueprint/Inventory/AC_Inventory.Try Add Item` InventoryComponent (`self.ItemObject`)))
  (`KismetSystemLibrary.PrintString` (`KismetStringLibrary.Conv_BoolToString` _added) true true (struct :`R` 1.0 :`B` 0.020422 :`A` 1.0))
  (if _added
    (`self.ServerDestroyItem`)))

(event `ServerDestroyItem`
  (`self.K2_DestroyActor`))

(fn `Get Default Item Object`
  (returns (ItemObject :type "/Game/Blueprint/Inventory/BP_BaseItemObject Object Reference"))
  (bind _returnvalue (`|GenericCreateObject` self "/Game/Blueprint/Inventory/BP_BaseItemObject.BP_BaseItemObject_C" (make `IntPoint` 2 1) "/Engine/EditorResources/BadBlueprintSprite.BadBlueprintSprite" "/Engine/EditorResources/BadBlueprintSprite.BadBlueprintSprite" (`GameplayStatics.GetObjectClass` self)))
  (return _returnvalue))

(fn `UserConstructionScript`)
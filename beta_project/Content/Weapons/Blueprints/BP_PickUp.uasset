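; World item pickup that shows a name widget to a nearby local player and is collected with E.
; OnRep_ID reads DT_Inventory, preferring DropItem data when set, then Update blocking-loads a skeletal mesh or falls back to static.
; Sphere overlap toggles widget and input for local players, and sets other characters as owner.
; A successful Character PickupItemMessage triggers DestroyServer to remove the actor.
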(event `self.ReceiveBeginPlay`
  ;[1 1 1] ID Changed
  (`self.OnRep_ID`))

(event `Key|E`
  (params (Key :type "Key Structure"))
  ;[1 1 1] PickUp
  (:`Pressed`
    (bind _success (message `/Game/Weapons/Blueprints/BPI_Inventory.PickupItem` (`self.Character`) (`self.ID`) (`self.Item`)))
    (if _success
      (`self.DestroyServer`))))

(event `DestroyServer`
  ;[1 1 1] Set server destroy actor
  (`self.K2_DestroyActor`))

(event `Update`
  (bind ((`DisplayName_19_53B795EB45F1F2B4C2A33EAF18B01F20` _displayname) (`PickupMesh_52_5430484D44B1B5CA13A6F4908B8F5AA0` _pickupmesh) (`PickupMeshStatic_50_85EC7FFF4F6A292B9ED92D81980E6B37` _pickupmeshstatic) (`HoldableSettings_51_3EBA43F549F1C0683E2A4BA60A35A7A8` _holdablesettings)) (break `/Game/Weapons/Data/ST_Inventory_Item` (`self.Item`)))
  ;[1 1 1] Update pickup item
  ;;[0 0.15 0.05531 0.5] set text widget
  (bind _aswbp_pickup (cast `/Game/Weapons/Widget/WBP_Pickup` (`WidgetComponent.GetWidget` (`self.Widget`))))
  (`TextBlock.SetText` (`/Game/Weapons/Widget/WBP_Pickup.TEXT` _aswbp_pickup) _displayname)
  ;;[0 0.15 0.05531 0.5] load skeletal mesh
  (bind _returnvalue (`KismetSystemLibrary.LoadAsset_Blocking` _pickupmesh))
  (bind _asskeletal_mesh (cast `SkeletalMesh` _returnvalue)
    (:`then`
      (`SkinnedMeshComponent.SetSkinnedAssetAndUpdate` (`self.SkeletalMesh`) _asskeletal_mesh true))
    (:`CastFailed`
      ;;[0 0.15 0.05531 0.5] set static mesh
      (bind _returnvalue_2 (`KismetSystemLibrary.LoadAsset_Blocking` _pickupmeshstatic))
      (cast `StaticMesh` _returnvalue_2)
      (`StaticMeshComponent.SetStaticMesh` (`self.StaticMesh`) null))))

(event `self.Sphere.OnComponentBeginOverlap`
  (params (OverlappedComponent :type "PrimitiveComponent Object Reference") (OtherActor :type "Actor Object Reference") (OtherComp :type "PrimitiveComponent Object Reference") (OtherBodyIndex :type Integer) (bFromSweep :type Boolean) (SweepResult :type "HitResult Structure (by ref)"))
  ;[1 1 1] Widget visible
  ;;[0 0.15 0.002229 0.5] Visible
  (bind _ascharacter (cast `Character` OtherActor))
  (bind _isnpc (`self.IsPlayer` _ascharacter)
    (:`true`
      (`SceneComponent.SetVisibility` (`self.Widget`) true false)
      ;[1 1 1] Enable interact key
      (`self.EnableInput` (`GameplayStatics.GetPlayerController` 0))
      ;[1 1 1] Create variable Character
      (set `self.Character` _ascharacter))
    (:`false`
      _))
  ;[1 1 1] Check is NPC
  (if (not _isnpc)
    (`self.SetOwner` _ascharacter)))

(event `self.Sphere.OnComponentEndOverlap`
  (params (OverlappedComponent :type "PrimitiveComponent Object Reference") (OtherActor :type "Actor Object Reference") (OtherComp :type "PrimitiveComponent Object Reference") (OtherBodyIndex :type Integer))
  ;[1 1 1] Widget visible
  ;;[0.15 0 0 0.5] Not visible
  (bind _ascharacter (cast `Character` OtherActor))
  (`self.IsPlayer` _ascharacter
    (:`true`
      (`SceneComponent.SetVisibility` (`self.Widget`) false false)
      ;[1 1 1] Enable interact key
      (`self.DisableInput` (`GameplayStatics.GetPlayerController` 0)))))

(fn `OnRep_ID`
  (bind _returnvalue (`|GetDataTableRow` "/Game/Weapons/DT_Inventory.DT_Inventory" (`self.ID`))
    (:`then`
      (set `self.Item` (select `bool` (!= (`.ID_46_56F388A54CD159E3A3F333915833CC03` (break `/Game/Weapons/Data/ST_Inventory_Item` (`self.DropItem`))) "None") :`false` _returnvalue :`true` (`self.DropItem`)))
      (`self.Update`))))

(fn `UserConstructionScript`)
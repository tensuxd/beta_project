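; BP_Weapon is a data-driven holdable weapon that takes its WeaponName from an overlapped BPI_Inventory actor.
; Construction and the WeaponName RepNotify call UpdateValues, which blocking-loads the DT_Inventory row's skeletal or fallback static mesh, fire settings, sound and VFX.
; FireON/FireOFF drive a Tick-fed Gate for automatic fire or a single shot, both rate-limited by DoOnce and Delay.
; Fire only plays sound, muzzle flash and debug text.
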(event `self.Sphere.OnComponentBeginOverlap`
  (params (OverlappedComponent :type "PrimitiveComponent Object Reference") (OtherActor :type "Actor Object Reference") (OtherComp :type "PrimitiveComponent Object Reference") (OtherBodyIndex :type Integer) (bFromSweep :type Boolean) (SweepResult :type "HitResult Structure (by ref)"))
  (if (`KismetSystemLibrary.DoesImplementInterface` OtherActor "/Game/Weapons/Blueprints/BPI_Inventory.BPI_Inventory_C")
    (bind _weaponname (message `/Game/Weapons/Blueprints/BPI_Inventory.Get Weapon Name` OtherActor))
    (set `self.WeaponName` _weaponname)
    (clear `self.OnActorBeginOverlap`)))

(event `self.ReceiveTick`
  (params (DeltaSeconds :type "Float (single-precision)"))
  (`/Engine/EditorBlueprintResources/StandardMacros.Gate` true :!label _label
    (:`Exit`
      (`KismetSystemLibrary.PrintString` "Hello")
      (`/Engine/EditorBlueprintResources/StandardMacros.DoOnce` false :!label _label_2
        (:`Completed`
          (`self.Fire`)
          (`KismetSystemLibrary.Delay` (`self.Fire Rate`))
          (goto _label_2 :!via `Reset`))))))

(event `/Game/Weapons/Blueprints/BPI_Weapon.FireON`
  (if (`self.Automatic`)
    (goto _label :!via `Open`)
    (else
      (goto _label_2))))

(event `/Game/Weapons/Blueprints/BPI_Weapon.FireOFF`
  (goto _label :!via `Close`))

(event `Fire`
  (`KismetSystemLibrary.PrintString` "Hello")
  (`GameplayStatics.PlaySoundAtLocation` (`self.FireSound`) (`self.K2_GetActorLocation`) (struct) 1.0 1.0 0.0 null null null null)
  (`GameplayStatics.SpawnEmitterAttached` (`self.FlashEmitter`) (`self.SkeletalMesh`) "TIP"))

(fn `Get Weapon Name`
  (returns (WeaponName :type Name))
  (return "None"))

(fn `OnRep_WeaponName`
  (`self.UpdateValues`))

(fn `Pick Up Weapon`
  (params (ID :type Name) (DropItem :type "/Game/Weapons/Data/ST_Inventory_Item Structure"))
  (returns (Success :type Boolean))
  (return false))

(fn `UpdateValues`
  (bind _returnvalue (`|GetDataTableRow` "/Game/Weapons/DT_Inventory.DT_Inventory" (`self.WeaponName`))
    (:`then`
      (bind ((`PickupMesh_52_5430484D44B1B5CA13A6F4908B8F5AA0` _pickupmesh) (`PickupMeshStatic_50_85EC7FFF4F6A292B9ED92D81980E6B37` _pickupmeshstatic) (`HoldableSettings_51_3EBA43F549F1C0683E2A4BA60A35A7A8` _holdablesettings)) (break `/Game/Weapons/Data/ST_Inventory_Item` _returnvalue))
      (bind _returnvalue_2 (`KismetSystemLibrary.LoadAsset_Blocking` _pickupmesh))
      (bind _asskeletal_mesh (cast `SkeletalMesh` _returnvalue_2)
        (:`then`
          (`SkinnedMeshComponent.SetSkinnedAssetAndUpdate` (`self.SkeletalMesh`) _asskeletal_mesh true))
        (:`CastFailed`
          (bind _returnvalue_3 (`KismetSystemLibrary.LoadAsset_Blocking` _pickupmeshstatic))
          (bind _asstatic_mesh (cast `StaticMesh` _returnvalue_3))
          (`StaticMeshComponent.SetStaticMesh` (`self.StaticMesh`) _asstatic_mesh)))
      (bind ((`Automatic_13_94F374CB4BDE9B6A914528BECBE54669` _automatic) (`FireRate_16_D80EC6814E1BFFA76A8FE9B76BA83FC7` _firerate) (`WeaponSound_22_A329B76348D879BD272339957C199418` _weaponsound) (`FireVFX_25_A0434012422AEFD40BF5AA81AEA2E0CB` _firevfx)) (break `/Game/Weapons/Data/ST_Inventory_Holdable` _holdablesettings))
      (set `self.Automatic` _automatic)
      (set `self.Fire Rate` _firerate)
      (bind _returnvalue_4 (`KismetSystemLibrary.LoadAsset_Blocking` _weaponsound))
      (bind _assound_base (cast `SoundBase` _returnvalue_4))
      (set `self.FireSound` _assound_base)
      (bind _returnvalue_5 (`KismetSystemLibrary.LoadAsset_Blocking` _firevfx))
      (bind _asparticle_system (cast `ParticleSystem` _returnvalue_5))
      (set `self.FlashEmitter` _asparticle_system))))

(fn `UserConstructionScript`
  (`self.UpdateValues`))